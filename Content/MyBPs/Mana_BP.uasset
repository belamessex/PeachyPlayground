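; Mana pickup actor that grants one mana to the player when BP_TPCharacter overlaps its static mesh.
; On overlap it calls AddMana, plays a pickup sound at its location and destroys itself.
; AddMana increments TotalMana on the PeachyPlayerState of player controller 0, regardless of which character touched it.
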(event OnComponentBeginOverlap(StaticMesh)
  (params (OverlappedComponent :type Primitive%20Component%20Object%20Reference) (OtherActor :type Actor%20Object%20Reference) (OtherComp :type Primitive%20Component%20Object%20Reference) (OtherBodyIndex :type Integer) (bFromSweep :type Boolean) (SweepResult :type Hit%20Result%20Structure%20%28by%20ref%29))
  (Utilities|Casting|CastToBP_TPCharacter OtherActor)
  (CallFunction|AddMana)
  (Audio|PlaySoundatLocation "/Game/MyAudio/Sep_fx_14.Sep_fx_14" (Transformation|GetActorLocation) "0, 0, 0" 1.0 1.0 0.0 0 0 0)
  (Actor|DestroyActor))

(event EventBeginPlay)

(event Collision|EventActorBeginOverlap
  (params (OtherActor :type Actor%20Object%20Reference)))

(event EventTick
  (params (DeltaSeconds :type Float%20%28single-precision%29)))

(fn ConstructionScript)

(fn AddMana
  (bind _aspeachy_player_state (Utilities|Casting|CastToPeachyPlayerState (Variables|/Script/Engine.Controller|GetPlayerState (Game|GetPlayerController 0))))
  (Variables|/Game/MyBPs/PeachyPlayerState.PeachyPlayerState_C|SetTotalMana _aspeachy_player_state (+ (Variables|/Game/MyBPs/PeachyPlayerState.PeachyPlayerState_C|GetTotalMana _aspeachy_player_state) 1)))