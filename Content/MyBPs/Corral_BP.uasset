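; Corral Blueprint with a door the player toggles open and closed by pressing Interact while standing in its trigger zone.
; PlayerChecker overlap with BP_TPCharacter enables or disables the actor's input for player controller 0.
; A FlipFlop plays or reverses the DoorMovement timeline, lerping the door's relative location between its starting position and the OpenDoorLoc marker at a configurable play rate.
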(event OnComponentBeginOverlap(PlayerChecker)
  (params (OverlappedComponent :type Primitive%20Component%20Object%20Reference) (OtherActor :type Actor%20Object%20Reference) (OtherComp :type Primitive%20Component%20Object%20Reference) (OtherBodyIndex :type Integer) (bFromSweep :type Boolean) (SweepResult :type Hit%20Result%20Structure%20%28by%20ref%29))
  ;[1 1 1] Enable/Disable Input
  (Utilities|Casting|CastToBP_TPCharacter OtherActor)
  (Input|EnableInput (Game|GetPlayerController 0)))

(event OnComponentEndOverlap(PlayerChecker)
  (params (OverlappedComponent :type Primitive%20Component%20Object%20Reference) (OtherActor :type Actor%20Object%20Reference) (OtherComp :type Primitive%20Component%20Object%20Reference) (OtherBodyIndex :type Integer))
  ;[1 1 1] Enable/Disable Input
  (Utilities|Casting|CastToBP_TPCharacter OtherActor)
  (Input|DisableInput (Game|GetPlayerController 0)))

(event EventBeginPlay
  ;[1 1 1] Get Initial variables
  (CallFunction|GetDoorLocations)
  (CallFunction|SetPlayRate))

(event Input|ActionEvents|InputActionInteract
  (params (Key :type Key%20Structure))
  ;[1 1 1] Toggle Door Position
  (:Pressed
    (Utilities|FlowControl|FlipFlop
      (:A
        (bind _newtrack_0 (Timeline|DoorMovement Play)
          (:Update
            (Transformation|SetRelativeLocation (Variables|Default|GetDoor) (Math|Vector|Lerp(Vector) (Variables|Default|GetClosedLoc) (Variables|Default|GetOpenLoc) _newtrack_0) false false))))
      (:B
        (Timeline|DoorMovement Reverse)))))

(fn ConstructionScript)

(fn GetDoorLocations
  (Variables|Default|SetClosedLoc (Variables|/Script/Engine.SceneComponent|GetRelativeLocation (Variables|Default|GetDoor)))
  (Variables|Default|SetOpenLoc (Variables|/Script/Engine.SceneComponent|GetRelativeLocation (Variables|Default|GetOpenDoorLoc))))

(fn SetPlayRate
  (Components|Timeline|SetPlayRate (Variables|Default|GetDoorMovement) (Variables|Default|GetDoorMoveRate)))