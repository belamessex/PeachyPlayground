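; Platform Blueprint set up to move a platform component between its starting position and an EndPoint component.
; BeginPlay caches both relative locations and sets the MovementTimeline play rate from MovementRate.
; The timeline's Update lerps the platform's relative location by MoveTime, without sweeping.
; No graph node starts the timeline, so movement depends on playback being triggered outside this graph, such as autoplay.
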(event EventBeginPlay
  ;[1 1 1] Get Locations
  (Variables|Default|SetStartLoc (Variables|/Script/Engine.SceneComponent|GetRelativeLocation (Variables|Default|GetPlatform)))
  (Variables|Default|SetEndLoc (Variables|/Script/Engine.SceneComponent|GetRelativeLocation (Variables|Default|GetEndPoint)))
  ;[1 1 1] Set Movement Rate
  (Components|Timeline|SetPlayRate (Variables|Default|GetMovement%20Timeline) (Variables|Default|GetMovementRate)))

(fn ConstructionScript)